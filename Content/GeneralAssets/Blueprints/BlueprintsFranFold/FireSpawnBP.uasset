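; FireSpawnBP is a pickup inventory item that spawns a FireSpawn actor at its DropLocation when used.
; Trigger overlaps show or remove a pickup text widget created on BeginPlay and track whether the item is in range.
; Its pickup event adds to the inventory, refreshes it, then hides the actor and disables collision.
; The binding for that event, widget text setup and custom mesh assignment are disconnected and never run.
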(event OnComponentBeginOverlap(Trigger)
  (params (OtherActor :type Actor%20Object%20Reference) (OtherComp :type Primitive%20Component%20Object%20Reference) (OtherBodyIndex :type Integer) (bFromSweep :type Boolean) (SweepResult :type Hit%20Result%20Structure%20%28by%20ref%29))
  ;[1 1 1] PickUpText Trigger
  (Utilities|Casting|CastTo OtherActor)
  (UserInterface|Viewport|AddtoViewport (Variables|Default|GetPickupTextReference) 0)
  (Variables|Default|SetIsinRange? true))

(event OnComponentEndOverlap(Trigger)
  (params (OtherActor :type Actor%20Object%20Reference) (OtherComp :type Primitive%20Component%20Object%20Reference) (OtherBodyIndex :type Integer))
  ;[1 1 1] PickUpText Trigger
  (Utilities|Casting|CastTo OtherActor)
  (Widget|RemovefromParent (Variables|Default|GetPickupTextReference))
  (Variables|Default|SetIsinRange? false))

(event Custom|PickUpItem_Event_0
  ;[1 1 1] PickUp and add items to inventory and refresh it
  (if (and (Collision|GetActorEnableCollision) (Variables|Default|GetIsinRange?))
    (Utilities|Array|Add :TargetArray (Variables|Default|GetInventory))
    (Widget|RemovefromParent (Variables|Default|GetPickupTextReference))
    (Rendering|SetActorHiddenInGame true)
    (Collision|SetActorEnableCollision false)
    (CallFunction|RefreshInventory)))

(event Custom|UseAction
  ;[1 1 1] Item Use Fuctionality
  (Game|SpawnActorfromClass "/Game/GeneralAssets/Blueprints/FireSpawn.FireSpawn_C" (Transformation|GetWorldTransform (Variables|Default|GetDropLocation)) "Undefined" 0 0))

(event EventBeginPlay
  ;[1 1 1] Event Begin Play
  (bind _returnvalue (UserInterface|CreateWidget "/Game/GeneralAssets/UMG/PickupText.PickupText_C"))
  (Variables|Default|SetPickupTextReference _returnvalue))

(fn ConstructionScript)