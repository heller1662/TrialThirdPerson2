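; Template inventory pickup actor that, when used, adjusts clamped health, energy and heart rate values, then destroys itself.
; BeginPlay creates a prompt widget, which trigger overlaps show or hide while setting an in-range flag.
; The pickup event adds to the inventory, removes the prompt, hides the actor without collision and refreshes the inventory.
; Pickup event binding, prompt setup and custom mesh assignment are disconnected, and cast targets are blank.
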(event OnComponentBeginOverlap(Trigger)
  (params (OtherActor :type Actor%20Object%20Reference) (OtherComp :type Primitive%20Component%20Object%20Reference) (OtherBodyIndex :type Integer) (bFromSweep :type Boolean) (SweepResult :type Hit%20Result%20Structure%20%28by%20ref%29))
  (bind _pickuptextreference (Variables|Default|GetPickupTextReference))
  ;[1 1 1] PickUpText Trigger
  (Utilities|Casting|CastTo OtherActor)
  (UserInterface|Viewport|AddtoViewport _pickuptextreference 0)
  (Widget|SetVisibility _pickuptextreference "Visible")
  (Variables|Default|SetIsinRange? true))

(event OnComponentEndOverlap(Trigger)
  (params (OtherActor :type Actor%20Object%20Reference) (OtherComp :type Primitive%20Component%20Object%20Reference) (OtherBodyIndex :type Integer))
  ;[1 1 1] PickUpText Trigger
  (Utilities|Casting|CastTo OtherActor)
  (Widget|SetVisibility (Variables|Default|GetPickupTextReference) "Hidden")
  (Variables|Default|SetIsinRange? false))

(event Custom|PickUpItem_Event_0
  ;[1 1 1] PickUp and add items to inventory and refresh it
  (if (and (Collision|GetActorEnableCollision) (Variables|Default|GetIsinRange?))
    (Utilities|Array|Add :TargetArray (Variables|Default|GetInventory))
    (Widget|RemovefromParent (Variables|Default|GetPickupTextReference))
    (Rendering|SetActorHiddenInGame true)
    (Collision|SetActorEnableCollision false)
    (CallFunction|RefreshInventory)))

(event Custom|UseAction
  ;[1 1 1] Item Use Fuctionality
  (Variables|Default|SetHealthValue (Math|Float|Clamp(Float) (+ (Variables|Default|GetHealthValue) (Variables|Default|GetaddHealth))))
  (Variables|Default|SetEnergyValue (Math|Float|Clamp(Float) (+ (Variables|Default|GetEnergyValue) (Variables|Default|GetaddEnergy))))
  (Variables|Default|SetHearthRateValue (Math|Float|Clamp(Float) (+ (Variables|Default|GetHearthRateValue) (Variables|Default|GetaddHearthRate))))
  (Actor|DestroyActor))

(event EventBeginPlay
  ;[1 1 1] Event Begin Play
  (bind _returnvalue (UserInterface|CreateWidget "/Game/GeneralAssets/UMG/PickupText.PickupText_C"))
  (Variables|Default|SetPickupTextReference _returnvalue))

(fn ConstructionScript)